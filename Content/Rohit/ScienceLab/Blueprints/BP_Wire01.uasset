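; BP_Wire01 is a configurable wire actor that builds spline meshes along its spline in the construction script.
; SplineMeshVar selects one segment per spline point pair or segments at fixed Spacing with scaled direction tangents.
; WireVar selects one of six segment variants, using one or two material slots, and WireSize scales each segment.
; Each segment gets dynamic MI_Wire instances driven by color, dirt, specular, roughness and a TextureVar-selected texture set.
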(fn ConstructionScript
  (|Wire))