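; Spawns a timed, colored smoke cloud from a pool of physics-driven static mesh components, each carrying an attached particle emitter.
; BeginPlay fills the pool at once or staggered, launching puffs along the Direction component.
; Tick, throttled by a delayed DoOnce, applies random dispersion and gravity forces.
; A recursive delayed timer recycles aged puffs to the spawn area, or destroys them once the smoke duration has elapsed.
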(event Custom|StopSmokeAfterDelay
  ;[0.875 0 1] Set Finished
  (Utilities|FlowControl|Delay (Variables|Settings|GetSmokeDuration))
  (Variables|Settings|SetFinished true))

(event Custom|SmokeDurationDestroy
  (bind _spawnradius (Variables|Movements|GetSpawnRadius))
  (bind _direction (Variables|Default|GetDirection))
  (bind _returnvalue (Transformation|GetWorldLocation _direction))
  ;[0.6406 1 0] Reset Pool Smoke
  (Utilities|FlowControl|Delay 0.1)
  (for (_array_element _array_index) (Variables|Infos|GetSmokeTimer)
    (if (>= _array_element (Variables|Settings|GetPoolResetTime))
      (Utilities|IsValid (Utilities|Array|Get(acopy) (Variables|Infos|GetSmokes) _array_index)
        (:Is%20Valid
          (Utilities|IsValid (Components|GetChildComponent (Utilities|Array|Get(acopy) (Variables|Infos|GetSmokes) _array_index) 0)
            (:Is%20Valid
              (Components|Activation|Deactivate (Components|GetChildComponent (Utilities|Array|Get(acopy) (Variables|Infos|GetSmokes) _array_index) 0)))
            (:Is%20Not%20Valid
              _))
          (if (Variables|Settings|GetFinished)
            (Components|DestroyComponent (Utilities|Array|Get(acopy) (Variables|Infos|GetSmokes) _array_index))
            (Utilities|Array|RemoveIndex (Variables|Infos|GetSmokeTimer) _array_index)
            (Utilities|Array|RemoveIndex (Variables|Infos|GetSmokes) _array_index)
            (else
              (Transformation|SetWorldLocation (Utilities|Array|Get(acopy) (Variables|Infos|GetSmokes) _array_index) (Math|Random|RandomPointinBoundingBox (Math|Vector|MakeVector (.x _returnvalue) (.y _returnvalue) (.z _returnvalue)) (Math|Vector|MakeVector _spawnradius _spawnradius 0.0)) false true)
              (Utilities|Array|SetArrayElem (Variables|Infos|GetSmokeTimer) _array_index 0.0 :!label _label)
              (Physics|AddForce (Utilities|Array|Get(acopy) (Variables|Infos|GetSmokes) _array_index) (* (Math|Vector|GetForwardVector (Variables|Default|GetDirection)) (* (* (Variables|Movements|GetBeginForce) 5e+04) (Math|Random|RandomFloatinRange 0.8 1.0))) "None" true)
              (bind _returnvalue_2 (Effects|SpawnEmitterAttached (Variables|Settings|GetEmitter) (Utilities|Array|Get(acopy) (Variables|Infos|GetSmokes) _array_index) "None" "0, 0, 0" "0, 0, 0" "1.000000,1.000000,1.000000" "SnapToTargetIncludingScale"))
              (Rendering|Material|SetMaterial _returnvalue_2 0 (Variables|Components|GetMaterial)))))
        (:Is%20Not%20Valid
          (goto _label)))
      (else
        (Utilities|Array|SetArrayElem (Variables|Infos|GetSmokeTimer) _array_index (+ _array_element 0.1)))))
  (CallFunction|SmokeDurationDestroy))

(event EventBeginPlay
  ;[0.3828 0 1] Init
  (CallFunction|StopSmokeAfterDelay)
  (CallFunction|InitColor)
  (CallFunction|SmokeDurationDestroy)
  (if (Variables|Settings|GetBurst?)
    (for _index (range 0 (Variables|Settings|GetPoolSize))
      (CallFunction|AddSmoke))
    (else
      (Utilities|ForLoopDelay 0 (Variables|Settings|GetPoolSize) (Variables|Settings|GetPoolSpawnDelay)
        (:Body
          (CallFunction|AddSmoke))))))

(event EventTick
  (params (DeltaSeconds :type Float%20%28single-precision%29))
  ;[1 0.9375 0] Movement
  (Utilities|FlowControl|DoOnce false :!label _label
    (:Completed
      (for _array_element (Variables|Infos|GetSmokes)
        (Utilities|IsValid _array_element
          (:Is%20Valid
            (Physics|AddForce _array_element (Math|Vector|MakeVector (.x (* (Math|Vector|GetForwardVector _array_element) (Math|Random|RandomFloatinRange (Variables|Movements|GetMinDispersion) (Variables|Movements|GetMaxDipsersion)))) (.y (* (Math|Vector|GetForwardVector _array_element) (Math|Random|RandomFloatinRange (Variables|Movements|GetMinDispersion) (Variables|Movements|GetMaxDipsersion)))) (* (* (Variables|Movements|GetGravity%20Force) (Math|Random|RandomFloatinRange 0.95 1.0)) 4.0)) "None" true))))
      (Utilities|FlowControl|Delay 0.1)
      (goto _label Reset))))

(fn ConstructionScript)

(fn InitColor
  (bind _returnvalue (Rendering|Material|CreateDynamicMaterialInstance (Variables|Settings|GetMaterialInstance) "None" "None" :!class /Script/Engine.KismetMaterialLibrary))
  (Variables|Components|SetMaterial _returnvalue)
  (Rendering|Material|SetVectorParameterValue _returnvalue "Color" (Variables|Settings|GetSmoke%20Color) :!class /Script/Engine.MaterialInstanceDynamic))

(fn AddSmoke
  (bind _damping (Variables|Physics|GetDamping))
  (bind _spawnradius (Variables|Movements|GetSpawnRadius))
  (bind _direction (Variables|Default|GetDirection))
  (bind _returnvalue (Transformation|GetWorldLocation _direction))
  (bind _returnvalue_2 (AddComponent|AddStaticMeshComponent true (Math|Transform|MakeTransform (Math|Random|RandomPointinBoundingBox (Math|Vector|MakeVector (.x _returnvalue) (.y _returnvalue) (.z _returnvalue)) (Math|Vector|MakeVector _spawnradius _spawnradius 0.0)) "0, 0, 0" (Math|Conversions|ToVector(Float) (Math|Random|RandomFloatinRange (Variables|Settings|GetMinScale) (Variables|Settings|GetMaxScale))))))
  (Rendering|SetVisibility _returnvalue_2 (Variables|Infos|GetDebug?) false)
  (Class|PrimitiveComponent|SetMassOverrideinKg _returnvalue_2 "None" (Variables|Physics|GetMass) true)
  (Class|PrimitiveComponent|SetAngularDamping _returnvalue_2 _damping)
  (Class|PrimitiveComponent|SetLinearDamping _returnvalue_2 _damping)
  (Utilities|Array|Add (Variables|Infos|GetSmokes) _returnvalue_2)
  (Utilities|Array|Add (Variables|Infos|GetSmokeTimer) 0.0)
  (Physics|AddForce _returnvalue_2 (* (Math|Vector|GetForwardVector (Variables|Default|GetDirection)) (* (* (Variables|Movements|GetBeginForce) 5e+04) (Math|Random|RandomFloatinRange 0.8 1.0))) "None" true)
  (bind _returnvalue_3 (Effects|SpawnEmitterAttached (Variables|Settings|GetEmitter) _returnvalue_2 "None" "0, 0, 0" "0, 0, 0" "1.000000,1.000000,1.000000" "SnapToTargetIncludingScale"))
  (Rendering|Material|SetMaterial _returnvalue_3 0 (Variables|Components|GetMaterial)))