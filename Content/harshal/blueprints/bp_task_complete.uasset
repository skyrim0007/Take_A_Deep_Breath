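; Task completion trigger actor that finishes an objective when the player's cop reaches it.
; When a Cop_BP whose CurrentTask matches this Task overlaps the alert box, it calls SlidOff on the cop, plays a completion sound and destroys itself.
; While MarkerEnable is set, Tick updates a marker widget with the player's distance in meters, caching the widget reference on first use.
; ToggleMarkerTask controls marker visibility and also runs at construction.
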(event OnComponentBeginOverlap(task_alert_box)
  (params (OverlappedComponent :type Primitive%20Component%20Object%20Reference) (OtherActor :type Actor%20Object%20Reference) (OtherComp :type Primitive%20Component%20Object%20Reference) (OtherBodyIndex :type Integer) (bFromSweep :type Boolean) (SweepResult :type Hit%20Result%20Structure%20%28by%20ref%29))
  (bind _ascop_bp (Utilities|Casting|CastToCop_BP OtherActor))
  (if (Utilities|Enum|Equal(Enum) (Variables|/Game/Priyanshu/Blueprint/Char_BP/Cop_BP.Cop_BP_C|Getcurrent_task _ascop_bp) (Variables|Default|Gettask))
    (Default|SlidOff _ascop_bp)
    (Audio|PlaySound2D "/Game/Fuyu/Final_Sounds/Objectives/Objective_Completed__1_25_.Objective_Completed__1_25_" 1.0 1.0 0.0 0 0)
    (Actor|DestroyActor)))

(event EventTick
  (params (DeltaSeconds :type Float%20%28single-precision%29))
  (if (Variables|Default|Getmarker%20enable)
    (CallFunction|UpdateMarkerPosition)
    (CallFunction|ToggleMarkerTask (Variables|Default|Getmarker%20enable))))

(fn ConstructionScript
  (CallFunction|ToggleMarkerTask (Variables|Default|Getmarker%20enable)))

(fn UpdateMarkerPosition
  (Variables|Default|Get%20Task%20Marker%20Widget%20ref
    (:then
      _)
    (:else
      (bind _astask_marker_widget (Utilities|Casting|CastTotask_marker_widget (UserInterface|GetUserWidgetObject (Variables|Default|Getmarker))))
      (Variables|Default|Set%20Task%20Marker%20Widget%20ref _astask_marker_widget)))
  (Default|UpdateText (Variables|Default|Get%20Task%20Marker%20Widget%20ref) (Utilities|String|Append (Utilities|String|ToString(Integer) (Math|Float|Round (/ (Math|Vector|Distance(Vector) (Transformation|GetActorLocation (Game|GetPlayerCharacter 0)) (Transformation|GetActorLocation)) 1e+02))) " m")))

(fn ToggleMarkerTask
  (params (bNewVisibility :type Boolean))
  (bind _output_get (Variables|Default|Setmarker%20enable bNewVisibility))
  (Rendering|SetVisibility (Variables|Default|Getmarker) _output_get false))