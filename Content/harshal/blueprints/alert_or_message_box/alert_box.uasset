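; Trigger actor that shows an alert message widget when the Cop_BP character enters its AlertBox component.
; Begin overlap stores the cop reference and, while the IsOverlaping flag is set, creates the Alert_message_widget and adds it to the viewport.
; End overlap clears the flag, waits briefly, then removes the widget and destroys the actor, so the alert is one-time.
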(event OnComponentBeginOverlap(alertbox)
  (params (OverlappedComponent :type Primitive%20Component%20Object%20Reference) (OtherActor :type Actor%20Object%20Reference) (OtherComp :type Primitive%20Component%20Object%20Reference) (OtherBodyIndex :type Integer) (bFromSweep :type Boolean) (SweepResult :type Hit%20Result%20Structure%20%28by%20ref%29))
  (bind _ascop_bp (Utilities|Casting|CastToCop_BP OtherActor))
  (Variables|Default|Set%20Cop%20BP%20ref _ascop_bp)
  (if (Variables|Default|Getis%20overlaping)
    (bind _returnvalue (UserInterface|CreateWidget "/Game/harshal/blueprints/alert_or_message_box/alert_message_widget.alert_message_widget_C"))
    (UserInterface|Viewport|AddtoViewport _returnvalue 0)))

(event OnComponentEndOverlap(alertbox)
  (params (OverlappedComponent :type Primitive%20Component%20Object%20Reference) (OtherActor :type Actor%20Object%20Reference) (OtherComp :type Primitive%20Component%20Object%20Reference) (OtherBodyIndex :type Integer))
  (Utilities|Casting|CastToCop_BP OtherActor)
  (Variables|Default|Setis%20overlaping false)
  (Utilities|FlowControl|Delay 2.0)
  (Widget|RemovefromParent (stale OnComponentBeginOverlap(alertbox) _returnvalue))
  (Actor|DestroyActor))

(event EventBeginPlay)

(event Collision|EventActorBeginOverlap
  (params (OtherActor :type Actor%20Object%20Reference)))

(event EventTick
  (params (DeltaSeconds :type Float%20%28single-precision%29)))

(fn ConstructionScript)