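; Pickup gas mask that the player's Cop_BP character can put on with an interact input.
; Box overlap stores the cop, opens a gate for the interact event and shows a key prompt, removed after two seconds or on exit.
; Interacting snaps the mask to the cop's HeadSocket if none is worn, sets WearingMask, plays a sound and destroys the trigger box.
; The gate is never closed when the cop leaves the box.
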(event OnComponentBeginOverlap(Box)
  (params (OverlappedComponent :type Primitive%20Component%20Object%20Reference) (OtherActor :type Actor%20Object%20Reference) (OtherComp :type Primitive%20Component%20Object%20Reference) (OtherBodyIndex :type Integer) (bFromSweep :type Boolean) (SweepResult :type Hit%20Result%20Structure%20%28by%20ref%29))
  (bind _ascop_bp (Utilities|Casting|CastToCop_BP OtherActor))
  (Variables|Default|Set%20Cop%20BP%20_ref _ascop_bp)
  (bind _returnvalue (UserInterface|CreateWidget "/Game/harshal/blueprints/widget_bp/interaction_key_widget.interaction_key_widget_C"))
  (UserInterface|Viewport|AddtoViewport _returnvalue 0)
  (Utilities|FlowControl|Sequence
    (:then_0
      (Utilities|FlowControl|Gate true) ; enters at Open
    )
    (:then_1
      (Utilities|FlowControl|Delay 2.0)
      (Widget|RemovefromParent _returnvalue))))

(event OnComponentEndOverlap(Box)
  (params (OverlappedComponent :type Primitive%20Component%20Object%20Reference) (OtherActor :type Actor%20Object%20Reference) (OtherComp :type Primitive%20Component%20Object%20Reference) (OtherBodyIndex :type Integer))
  (Utilities|Casting|CastToCop_BP OtherActor)
  (Widget|RemovefromParent (stale OnComponentBeginOverlap(Box) _returnvalue)))

(event EventExpertInteract
  (Utilities|FlowControl|Gate true
    (:Exit
      (if (not (Variables|/Game/Priyanshu/Blueprint/Char_BP/Cop_BP.Cop_BP_C|GetWearing%20Mask (Variables|Default|Get%20Cop%20BP%20_ref)))
        (Transformation|AttachComponentToComponent (Variables|/Script/Engine.Character|GetMesh (Variables|Default|Get%20Cop%20BP%20_ref)) "HeadSocket" "SnapToTarget" "SnapToTarget" "SnapToTarget" true)
        (Variables|/Game/Priyanshu/Blueprint/Char_BP/Cop_BP.Cop_BP_C|SetWearing%20Mask (Variables|Default|Get%20Cop%20BP%20_ref) true)
        (Audio|PlaySound2D "/Game/Fuyu/Final_Sounds/Gas_Mask/Gas_Mask_Take_off__1_12_s_.Gas_Mask_Take_off__1_12_s_" 1.0 1.0 0.0 0 0)
        (Widget|RemovefromParent (stale OnComponentBeginOverlap(Box) _returnvalue))
        (Components|DestroyComponent (Variables|Default|GetBox))))))

(fn ConstructionScript)