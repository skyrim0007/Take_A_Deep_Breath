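; Readable document actor that lets the player open and close a document widget with the ExpertInteract event.
; A trigger box shows an interaction key widget when Cop_BP enters and removes it on exit.
; ExpertInteract uses a FlipFlop to alternately create and remove the document widget.
; Player input is enabled at BeginPlay and disabled when the cop leaves the box, with no re-enable on re-entry.
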(event OnComponentBeginOverlap(triggerbox)
  (params (OverlappedComponent :type Primitive%20Component%20Object%20Reference) (OtherActor :type Actor%20Object%20Reference) (OtherComp :type Primitive%20Component%20Object%20Reference) (OtherBodyIndex :type Integer) (bFromSweep :type Boolean) (SweepResult :type Hit%20Result%20Structure%20%28by%20ref%29))
  (bind _ascop_bp (Utilities|Casting|CastToCop_BP OtherActor))
  (Variables|Default|Set%20Cop%20BP%20ref _ascop_bp)
  (bind _returnvalue (UserInterface|CreateWidget "/Game/harshal/blueprints/widget_bp/interaction_key_widget.interaction_key_widget_C"))
  (UserInterface|Viewport|AddtoViewport _returnvalue 0))

(event OnComponentEndOverlap(triggerbox)
  (params (OverlappedComponent :type Primitive%20Component%20Object%20Reference) (OtherActor :type Actor%20Object%20Reference) (OtherComp :type Primitive%20Component%20Object%20Reference) (OtherBodyIndex :type Integer))
  (Utilities|Casting|CastToCop_BP OtherActor)
  (Widget|RemovefromParent (stale OnComponentBeginOverlap(triggerbox) _returnvalue))
  (Input|DisableInput (Game|GetPlayerController 0)))

(event EventBeginPlay
  (Input|EnableInput (Game|GetPlayerController 0)))

(event Collision|EventActorBeginOverlap
  (params (OtherActor :type Actor%20Object%20Reference)))

(event EventTick
  (params (DeltaSeconds :type Float%20%28single-precision%29)))

(event EventExpertInteract
  (Utilities|FlowControl|FlipFlop
    (:A
      (bind _returnvalue (UserInterface|CreateWidget "/Game/harshal/blueprints/reading_document/document_widget.document_widget_C"))
      (UserInterface|Viewport|AddtoViewport _returnvalue 0))
    (:B
      (Widget|RemovefromParent _returnvalue))))

(fn ConstructionScript)