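; Secret door actor that slides open when interacted with and closes itself once the player cop leaves.
; A Cop_BP entering the box opens a gate that lets ExpertInteract through; nothing closes that gate again.
; Interacting while the door is shut plays a sound and a timeline that slides the mesh along local Y.
; Leaving the box while it is open replays the sound and reverses the timeline.
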(event OnComponentBeginOverlap(Box)
  (params (OverlappedComponent :type Primitive%20Component%20Object%20Reference) (OtherActor :type Actor%20Object%20Reference) (OtherComp :type Primitive%20Component%20Object%20Reference) (OtherBodyIndex :type Integer) (bFromSweep :type Boolean) (SweepResult :type Hit%20Result%20Structure%20%28by%20ref%29))
  ;[0 0 0 1 30] door mechanics
  (bind _ascop_bp (Utilities|Casting|CastToCop_BP OtherActor))
  (Variables|Default|Set%20Cop%20BP%20ref _ascop_bp)
  (Utilities|FlowControl|Gate true) ; enters at Open
)

(event OnComponentEndOverlap(Box)
  (params (OverlappedComponent :type Primitive%20Component%20Object%20Reference) (OtherActor :type Actor%20Object%20Reference) (OtherComp :type Primitive%20Component%20Object%20Reference) (OtherBodyIndex :type Integer))
  ;[0 0 0 1 30] door mechanics
  (Utilities|Casting|CastToCop_BP OtherActor)
  (if (Variables|Default|Getis%20open?)
    (Audio|PlaySoundatLocation "/Game/Fuyu/Final_Sounds/Door/Automatic_Door_Open__2_00_s_.Automatic_Door_Open__2_00_s_" (Variables|/Script/Engine.SceneComponent|GetRelativeLocation (Variables|Default|Getdoor)) "0, 0, 0" 1.0 1.0 0.0 0 0 0 0)
    (Variables|Default|Setis%20open? false)
    (bind _door (Timeline|door%20opening Reverse)
      (:Update
        (Transformation|SetRelativeLocation (Variables|Default|Getdoor) (Math|Vector|MakeVector 0.0 (Math|Float|Lerp 0.0 2.7e+02 _door) 0.0) false false)))))

(event EventBeginPlay)

(event Collision|EventActorBeginOverlap
  (params (OtherActor :type Actor%20Object%20Reference)))

(event EventTick
  (params (DeltaSeconds :type Float%20%28single-precision%29)))

(event EventExpertInteract
  ;[0 0 0 1 30] door mechanics
  (if (not (Variables|Default|Getis%20open?))
    (Utilities|FlowControl|Gate true
      (:Exit
        (Variables|Default|Setis%20open? true)
        (Audio|PlaySoundatLocation "/Game/Fuyu/Final_Sounds/Door/Automatic_Door_Open__2_00_s_.Automatic_Door_Open__2_00_s_" (Variables|/Script/Engine.SceneComponent|GetRelativeLocation (Variables|Default|Getdoor)) "0, 0, 0" 1.0 1.0 0.0 0 0 0 0)
        (bind _door (Timeline|door%20opening Play)
          (:Update
            (Transformation|SetRelativeLocation (Variables|Default|Getdoor) (Math|Vector|MakeVector 0.0 (Math|Float|Lerp 0.0 2.7e+02 _door) 0.0) false false)))))))

(fn ConstructionScript)