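; Automatic single sliding door that opens when something overlaps its Box trigger and closes when the overlap ends.
; The DoorOpening timeline plays forward on begin overlap and reverses on end overlap, lerping the Door component's relative Y position to slide it.
; Both transitions play the same door-open sound, positioned using the door's relative location rather than its world location.
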(event OnComponentBeginOverlap(Box)
  (params (OverlappedComponent :type Primitive%20Component%20Object%20Reference) (OtherActor :type Actor%20Object%20Reference) (OtherComp :type Primitive%20Component%20Object%20Reference) (OtherBodyIndex :type Integer) (bFromSweep :type Boolean) (SweepResult :type Hit%20Result%20Structure%20%28by%20ref%29))
  ;[0 0 0 1 30] door mechanics
  (Audio|PlaySoundatLocation "/Game/Fuyu/Final_Sounds/Door/Automatic_Door_Open__2_00_s_.Automatic_Door_Open__2_00_s_" (Variables|/Script/Engine.SceneComponent|GetRelativeLocation (Variables|Default|Getdoor)) "0, 0, 0" 1.0 1.0 0.0 0 0 0 0)
  (bind _door (Timeline|door%20opening Play)
    (:Update
      (Transformation|SetRelativeLocation (Variables|Default|Getdoor) (Math|Vector|MakeVector 0.0 (Math|Float|Lerp 0.0 2e+02 _door) 0.0) false false))))

(event OnComponentEndOverlap(Box)
  (params (OverlappedComponent :type Primitive%20Component%20Object%20Reference) (OtherActor :type Actor%20Object%20Reference) (OtherComp :type Primitive%20Component%20Object%20Reference) (OtherBodyIndex :type Integer))
  ;[0 0 0 1 30] door mechanics
  (Audio|PlaySoundatLocation "/Game/Fuyu/Final_Sounds/Door/Automatic_Door_Open__2_00_s_.Automatic_Door_Open__2_00_s_" (Variables|/Script/Engine.SceneComponent|GetRelativeLocation (Variables|Default|Getdoor)) "0, 0, 0" 1.0 1.0 0.0 0 0 0 0)
  (bind _door (Timeline|door%20opening Reverse)
    (:Update
      (Transformation|SetRelativeLocation (Variables|Default|Getdoor) (Math|Vector|MakeVector 0.0 (Math|Float|Lerp 0.0 2e+02 _door) 0.0) false false))))

(event EventBeginPlay)

(event Collision|EventActorBeginOverlap
  (params (OtherActor :type Actor%20Object%20Reference)))

(event EventTick
  (params (DeltaSeconds :type Float%20%28single-precision%29)))

(fn ConstructionScript)