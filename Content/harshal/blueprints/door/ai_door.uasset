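; Sliding double door Blueprint (ai_door) that opens and closes through a box trigger.
; Begin overlap plays two timelines that lerp the left and right leaves apart along relative Y, but only when the overlapping actor casts to bp_double_door.
; End overlap reverses both timelines to close the leaves, with no check on which actor left.
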(event OnComponentBeginOverlap(Box)
  (params (OverlappedComponent :type Primitive%20Component%20Object%20Reference) (OtherActor :type Actor%20Object%20Reference) (OtherComp :type Primitive%20Component%20Object%20Reference) (OtherBodyIndex :type Integer) (bFromSweep :type Boolean) (SweepResult :type Hit%20Result%20Structure%20%28by%20ref%29))
  (Utilities|Casting|CastTobp_double_door OtherActor)
  (Utilities|FlowControl|Sequence
    (:then_0
      (bind _open_door (Timeline|right%20door Play)
        (:Update
          (Transformation|SetRelativeLocation (Variables|Default|Getright%20door) (Math|Vector|MakeVector 0.0 (Math|Float|Lerp -5e+01 -1.5e+02 _open_door) 0.0) false false))))
    (:then_1
      (bind _open_door_2 (Timeline|left%20door Play)
        (:Update
          (Transformation|SetRelativeLocation (Variables|Default|Getleft%20door) (Math|Vector|MakeVector 0.0 (Math|Float|Lerp 5e+01 1.5e+02 _open_door_2) 0.0) false false))))))

(event OnComponentEndOverlap(Box)
  (params (OverlappedComponent :type Primitive%20Component%20Object%20Reference) (OtherActor :type Actor%20Object%20Reference) (OtherComp :type Primitive%20Component%20Object%20Reference) (OtherBodyIndex :type Integer))
  (Utilities|FlowControl|Sequence
    (:then_0
      (bind _open_door (Timeline|right%20door Reverse)
        (:Update
          (Transformation|SetRelativeLocation (Variables|Default|Getright%20door) (Math|Vector|MakeVector 0.0 (Math|Float|Lerp -5e+01 -1.5e+02 _open_door) 0.0) false false))))
    (:then_1
      (bind _open_door_2 (Timeline|left%20door Reverse)
        (:Update
          (Transformation|SetRelativeLocation (Variables|Default|Getleft%20door) (Math|Vector|MakeVector 0.0 (Math|Float|Lerp 5e+01 1.5e+02 _open_door_2) 0.0) false false))))))

(event EventBeginPlay)

(event Collision|EventActorBeginOverlap
  (params (OtherActor :type Actor%20Object%20Reference)))

(event EventTick
  (params (DeltaSeconds :type Float%20%28single-precision%29)))

(fn ConstructionScript)