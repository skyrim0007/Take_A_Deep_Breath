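; Key-card-locked sliding double door that opens for the player's Cop_BP.
; On box overlap it checks HaveKey on the level's Door_key_card, then plays a sound and timelines that slide both panels apart, or briefly shows a key message widget.
; Leaving the box with the key reverses the timelines with a closing sound.
; A separate doorsuddenlyclosed event uses its own timelines to slide the panels shut, playing the opening sound.
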(event OnComponentBeginOverlap(Box)
  (params (OverlappedComponent :type Primitive%20Component%20Object%20Reference) (OtherActor :type Actor%20Object%20Reference) (OtherComp :type Primitive%20Component%20Object%20Reference) (OtherBodyIndex :type Integer) (bFromSweep :type Boolean) (SweepResult :type Hit%20Result%20Structure%20%28by%20ref%29))
  (bind _ascop_bp (Utilities|Casting|CastToCop_BP OtherActor))
  (Variables|Default|Set%20Cop%20BP%20ref _ascop_bp)
  (bind _returnvalue (Actor|GetActorOfClass "/Game/harshal/blueprints/door/special_doors/double_door_with_key/door_key_card.door_key_card_C"))
  (if (Variables|/Game/harshal/blueprints/door/special_doors/double_door_with_key/door_key_card.door_key_card_C|Gethave%20key%20? _returnvalue)
    (Audio|PlaySoundatLocation "/Game/Fuyu/Final_Sounds/Door/Metal_Door_Open__2_91_s_.Metal_Door_Open__2_91_s_" (Transformation|GetActorLocation) "0, 0, 0" 1.0 1.0 0.0 0 0 0 0)
    (Utilities|FlowControl|Sequence
      (:then_0
        (bind _open_door (Timeline|right%20door Play)
          (:Update
            (Transformation|SetRelativeLocation (Variables|Default|Getright%20door) (Math|Vector|MakeVector 0.0 (Math|Float|Lerp -62.0 -1.5e+02 _open_door) 0.0) false false))))
      (:then_1
        (bind _open_door_2 (Timeline|left%20door Play)
          (:Update
            (Transformation|SetRelativeLocation (Variables|Default|Getleft%20door) (Math|Vector|MakeVector 0.0 (Math|Float|Lerp 62.0 1.5e+02 _open_door_2) 0.0) false false)))))
    (else
      (bind _returnvalue_2 (UserInterface|CreateWidget "/Game/harshal/blueprints/door/special_doors/double_door_with_key/door_key_message.door_key_message_C"))
      (UserInterface|Viewport|AddtoViewport _returnvalue_2 0)
      (Utilities|FlowControl|Delay 2.0)
      (Widget|RemovefromParent _returnvalue_2))))

(event OnComponentEndOverlap(Box)
  (params (OverlappedComponent :type Primitive%20Component%20Object%20Reference) (OtherActor :type Actor%20Object%20Reference) (OtherComp :type Primitive%20Component%20Object%20Reference) (OtherBodyIndex :type Integer))
  (Utilities|Casting|CastToCop_BP OtherActor)
  (if (Variables|/Game/harshal/blueprints/door/special_doors/double_door_with_key/door_key_card.door_key_card_C|Gethave%20key%20? (stale OnComponentBeginOverlap(Box) _returnvalue))
    (Audio|PlaySoundatLocation "/Game/Fuyu/Final_Sounds/Door/Metal_Slide_Door_close__2_91_s_.Metal_Slide_Door_close__2_91_s_" (Transformation|GetActorLocation) "0, 0, 0" 1.0 1.0 0.0 0 0 0 0)
    (Utilities|FlowControl|Sequence
      (:then_0
        (bind _open_door (Timeline|right%20door Reverse)
          (:Update
            (Transformation|SetRelativeLocation (Variables|Default|Getright%20door) (Math|Vector|MakeVector 0.0 (Math|Float|Lerp -62.0 -1.5e+02 _open_door) 0.0) false false))))
      (:then_1
        (bind _open_door_2 (Timeline|left%20door Reverse)
          (:Update
            (Transformation|SetRelativeLocation (Variables|Default|Getleft%20door) (Math|Vector|MakeVector 0.0 (Math|Float|Lerp 62.0 1.5e+02 _open_door_2) 0.0) false false)))))))

(event Custom|door%20suddenly%20closed
  (Utilities|FlowControl|Sequence
    (:then_0
      (Audio|PlaySoundatLocation "/Game/Fuyu/Final_Sounds/Door/Metal_Door_Open__2_91_s_.Metal_Door_Open__2_91_s_" (Transformation|GetActorLocation) "0, 0, 0" 1.0 1.0 0.0 0 0 0 0)
      (bind _open_door (Timeline|Timeline_0 Play)
        (:Update
          (Transformation|SetRelativeLocation (Variables|Default|Getright%20door) (Math|Vector|MakeVector 0.0 (Math|Float|Lerp -1.5e+02 -5e+01 _open_door) 0.0) false false))))
    (:then_1
      (bind _open_door_2 (Timeline|Timeline_1 Play)
        (:Update
          (Transformation|SetRelativeLocation (Variables|Default|Getleft%20door) (Math|Vector|MakeVector 0.0 (Math|Float|Lerp 1.5e+02 5e+01 _open_door_2) 0.0) false false))))))

(event EventBeginPlay)

(event Collision|EventActorBeginOverlap
  (params (OtherActor :type Actor%20Object%20Reference)))

(event EventTick
  (params (DeltaSeconds :type Float%20%28single-precision%29)))

(fn ConstructionScript)