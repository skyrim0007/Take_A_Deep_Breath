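; Interactive single sliding door that the Cop_BP character can open and close while standing inside its trigger box.
; Box overlap by the cop shows an interaction key widget and opens a gate; ending overlap removes the widget and closes the gate.
; While the gate is open, the ExpertInteract event flip-flops the DoorOpening timeline between play and reverse, lerping the door's relative X location to slide it.
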(event OnComponentBeginOverlap(Box)
  (params (OverlappedComponent :type Primitive%20Component%20Object%20Reference) (OtherActor :type Actor%20Object%20Reference) (OtherComp :type Primitive%20Component%20Object%20Reference) (OtherBodyIndex :type Integer) (bFromSweep :type Boolean) (SweepResult :type Hit%20Result%20Structure%20%28by%20ref%29))
  ;[0 0 0 1 30] door mechanics
  (bind _ascop_bp (Utilities|Casting|CastToCop_BP OtherActor))
  (Variables|Default|Set%20Cop%20BP%20ref _ascop_bp)
  (bind _returnvalue (UserInterface|CreateWidget "/Game/harshal/blueprints/widget_bp/interaction_key_widget.interaction_key_widget_C"))
  (UserInterface|Viewport|AddtoViewport _returnvalue 0)
  (Utilities|FlowControl|Gate true) ; enters at Open
)

(event OnComponentEndOverlap(Box)
  (params (OverlappedComponent :type Primitive%20Component%20Object%20Reference) (OtherActor :type Actor%20Object%20Reference) (OtherComp :type Primitive%20Component%20Object%20Reference) (OtherBodyIndex :type Integer))
  ;[0 0 0 1 30] door mechanics
  (Widget|RemovefromParent (stale OnComponentBeginOverlap(Box) _returnvalue))
  (Utilities|FlowControl|Gate true) ; enters at Close
)

(event EventBeginPlay
  (Input|EnableInput (Game|GetPlayerController 0)))

(event Collision|EventActorBeginOverlap
  (params (OtherActor :type Actor%20Object%20Reference)))

(event EventTick
  (params (DeltaSeconds :type Float%20%28single-precision%29)))

(event EventExpertInteract
  ;[0 0 0 1 30] door mechanics
  (Utilities|FlowControl|Gate true
    (:Exit
      (Utilities|FlowControl|FlipFlop
        (:A
          (bind _door (Timeline|door%20opening Play)
            (:Update
              (Transformation|SetRelativeLocation (Variables|Default|Getdoor) (Math|Vector|MakeVector (Math|Float|Lerp 0.0 -2e+02 _door) 0.0 0.0) false false))))
        (:B
          (Timeline|door%20opening Reverse))))))

(fn ConstructionScript)