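; Cop_BP is a player-controllable character Blueprint, named for a cop, that handles basic movement and look input.
; Axis inputs move it along directions derived from actor rotation and feed controller pitch and yaw for looking.
; Sprint doubles the CharacterMovement max walk speed while held, and Crouch uses the built-in crouch and uncrouch on press and release.
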(event Input|ActionEvents|InputActionSprint
  (params (Key :type Key%20Structure :default "None"))
  (bind _charactermovement (Variables|Character|GetCharacterMovement))
  ;[0.0131 0 1 1 32] Sprint
  (:Pressed
    (Variables|/Script/Engine.CharacterMovementComponent|SetMaxWalkSpeed _charactermovement 8e+02))
  (:Released
    (Variables|/Script/Engine.CharacterMovementComponent|SetMaxWalkSpeed _charactermovement 4e+02)))

(event Input|ActionEvents|InputActionCrouch
  (params (Key :type Key%20Structure :default "None"))
  ;[0.04251 0 1 1 32] Crouch
  (:Pressed
    (Character|Crouch))
  (:Released
    (Character|UnCrouch)))

(event Input|AxisEvents|InputAxisMoveForward/Backward
  (params (AxisValue :type Float%20%28single-precision%29))
  ;[0.04458 0 1 1 32] Movement
  (Pawn|Input|AddMovementInput (Math|Vector|GetForwardVector (Math|Rotator|MakeRotator 0.0 0.0 (.yaw (Transformation|GetActorRotation)))) AxisValue false))

(event Input|AxisEvents|InputAxisMoveRight/Left
  (params (AxisValue :type Float%20%28single-precision%29))
  (bind _returnvalue (Transformation|GetActorRotation))
  ;[0.04458 0 1 1 32] Movement
  (Pawn|Input|AddMovementInput (Math|Vector|GetRightVector (Math|Rotator|MakeRotator (.roll _returnvalue) 0.0 (.yaw _returnvalue))) AxisValue false))

(event Input|AxisEvents|InputAxisLookUp/Down
  (params (AxisValue :type Float%20%28single-precision%29))
  ;[0.07481 0 1 1 32] Look
  (Pawn|Input|AddControllerPitchInput AxisValue))

(event Input|AxisEvents|InputAxisLookLeft/Right
  (params (AxisValue :type Float%20%28single-precision%29))
  ;[0.07481 0 1 1 32] Look
  (Pawn|Input|AddControllerYawInput AxisValue))

(fn ConstructionScript)