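; Capsule cell actor that the player opens to rescue someone, with the final rescue starting a poison gas leak.
; ExpertInteract swings the door via a flip-flopped timeline, destroys the cylinder, decrements Cop_Gamemode's RescuedPerson count and shows a rescue widget.
; At zero it removes that widget, activates the smoke spawner, shows a countdown widget and moves the damage box into place after a delay.
; A self-calling Delay event counts up elapsed minutes and seconds.
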(event Custom|OpenDoor
  (Utilities|FlowControl|FlipFlop
    (:A
      (bind _movement (Timeline|Open/close Play)
        (:Update
          (Transformation|SetRelativeRotation (Variables|Default|GetDoor) (Math|Rotator|MakeRotator 0.0 0.0 (* _movement 9e+01)) false false))))
    (:B
      (Timeline|Open/close Reverse))))

(event Custom|timer
  ;[0 0 0 1 30] timer
  (Utilities|FlowControl|Delay 1.0)
  (Variables|timeercountdownvariables|Settime%20sec (+ (Variables|timeercountdownvariables|Gettime%20sec) 1.0))
  (if (> (Variables|timeercountdownvariables|Gettime%20sec) 59.0)
    (Variables|timeercountdownvariables|Settime%20min (+ (Variables|timeercountdownvariables|Gettime%20min) 1.0))
    (Variables|timeercountdownvariables|Settime%20sec 0.0)
    (CallFunction|Timer)
    (else
      (CallFunction|Timer))))

(event EventExpertInteract
  (CallFunction|OpenDoor)
  (Utilities|FlowControl|Delay 1.0)
  (Components|DestroyComponent (Variables|Default|GetCylinder))
  (Utilities|FlowControl|Delay 0.2)
  (bind _ascop_gamemode (Utilities|Casting|CastToCop_Gamemode (Game|GetGameMode)))
  (bind _result (Math|Integer|DecrementInt (Variables|/Game/Priyanshu/Blueprint/Char_BP/Cop_Gamemode.Cop_Gamemode_C|Getrescued%20person _ascop_gamemode))
    (:%20%20
      (bind _output_get (Variables|/Game/Priyanshu/Blueprint/Char_BP/Cop_Gamemode.Cop_Gamemode_C|Setrescued%20person _ascop_gamemode _result))
      (bind _returnvalue (UserInterface|CreateWidget "/Game/Priyanshu/widget/Rescued_widget.Rescued_widget_C"))
      (UserInterface|Viewport|AddtoViewport _returnvalue 0)
      (if (== _output_get 0)
        (Utilities|FlowControl|Delay 0.2)
        ;[0 0 0 1 30] poison spawning logic
        (Widget|RemovefromParent _returnvalue)
        (Development|PrintString "gas leak start" true true "(R=1.000000,G=0.033493,B=0.000000,A=1.000000)")
        (bind _returnvalue_2 (Actor|GetActorOfClass "/Game/harshal/niagara/poison_smoke_spwaner.poison_smoke_spwaner_C"))
        (bind _output_get_2 (Variables|poisonvariables|Setpoison_smoke_spwaner _returnvalue_2))
        (Components|Activation|Activate (Variables|/Game/harshal/niagara/poison_smoke_spwaner.poison_smoke_spwaner_C|Getsmoke%20spwaner _output_get_2) false)
        (bind _returnvalue_3 (UserInterface|CreateWidget "/Game/harshal/blueprints/widget_bp/timer_countdown.timer_countdown_C"))
        (UserInterface|Viewport|AddtoViewport _returnvalue_3 0)
        (CallFunction|Timer)
        (Utilities|FlowControl|Delay 3.0)
        (bind _returnvalue_4 (Actor|GetActorOfClass "/Game/harshal/blueprints/poison_smoke_damage_box.poison_smoke_damage_box_C"))
        (Transformation|SetActorLocation _returnvalue_4 (Variables|PoisonVariables|Getpoison%20box%20location) false false)
        (else
          (Development|PrintString "no" true true "(R=0.276810,G=0.415379,B=1.000000,A=1.000000)"))))))

(fn ConstructionScript)