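; Armed NPC that roams to random reachable points and attacks the player-type Cop_BP pawn on sight.
; Roaming restarts only on successful moves; PawnSensing sightings make it face and approach the cop, firing bullets with a montage behind a delay gate that also toggles walk speed.
; A sphere overlap moves it toward a cop whose IsBreathing is set.
; The waypoint-chain AI_Patrol graph is not called from the event graph.
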(event OnSeePawn(PawnSensing)
  (params (Pawn :type Pawn%20Object%20Reference))
  (bind _ascop_bp (Utilities|Casting|CastToCop_BP Pawn))
  (Utilities|FlowControl|Sequence
    (:then_0
      (Transformation|SetActorRotation (Math|Rotator|FindLookatRotation (Transformation|GetActorLocation) (Transformation|GetActorLocation _ascop_bp)))
      (AI|AIMoveTo self "0, 0, 0" _ascop_bp 5e+02 false))
    (:then_1
      (if (Variables|Default|GetSHOOT%20DELAY)
        (Animation|PlayAnimMontage "/Game/Adi/AI/Animations/Firing_Rifle1_Montage.Firing_Rifle1_Montage" 1.0 "None")
        (Variables|/Script/Engine.CharacterMovementComponent|SetMaxWalkSpeed (Variables|Character|GetCharacterMovement) 1e+02)
        (Game|SpawnActorfromClass "/Game/Harsh_AI_wala/BULLETS.BULLETS_C" (Transformation|GetWorldTransform (Variables|Default|GetScene)) "Undefined" 0 0)
        (Variables|Default|SetSHOOT%20DELAY false)
        (Utilities|FlowControl|Delay 0.3)
        (Variables|Default|SetSHOOT%20DELAY true)
        (else
          (Variables|/Script/Engine.CharacterMovementComponent|SetMaxWalkSpeed (Variables|Character|GetCharacterMovement) 3e+02))))))

(event OnComponentBeginOverlap(Sphere)
  (params (OverlappedComponent :type Primitive%20Component%20Object%20Reference) (OtherActor :type Actor%20Object%20Reference) (OtherComp :type Primitive%20Component%20Object%20Reference) (OtherBodyIndex :type Integer) (bFromSweep :type Boolean) (SweepResult :type Hit%20Result%20Structure%20%28by%20ref%29))
  (bind _ascop_bp (Utilities|Casting|CastToCop_BP OtherActor))
  (if (Variables|/Game/Priyanshu/Blueprint/Char_BP/Cop_BP.Cop_BP_C|Getis%20%20breathing%20? _ascop_bp)
    (AI|AIMoveTo self "0, 0, 0" _ascop_bp 1.5e+02 false)))

(event Custom|Random_Rom
  (AI|AIMoveTo self (.RandomLocation (AI|Navigation|GetRandomReachablePointinRadius (Transformation|GetActorLocation) 2.5e+03 0 0)) 0 5.0 false
    (:OnSuccess
      (CallFunction|RandomRom))))

(event EventBeginPlay
  (CallFunction|RandomRom))

(event Collision|EventActorBeginOverlap
  (params (OtherActor :type Actor%20Object%20Reference)))

(event EventTick
  (params (DeltaSeconds :type Float%20%28single-precision%29)))

(fn ConstructionScript)